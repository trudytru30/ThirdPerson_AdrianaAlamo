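; BP_Door is a sliding double stone door that stays locked until its Interaction event sets Active.
; When BP_Ninja enters the Box while active, it collapses the HUD key icon and plays a timeline that moves both leaves apart on X, reversing on exit.
; While locked, entering plays an interact sound and shows a TextRender, which hides again on exit.
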(event OnComponentBeginOverlap(Box)
  (params (OverlappedComponent :type Primitive%20Component%20Object%20Reference) (OtherActor :type Actor%20Object%20Reference) (OtherComp :type Primitive%20Component%20Object%20Reference) (OtherBodyIndex :type Integer) (bFromSweep :type Boolean) (SweepResult :type Hit%20Result%20Structure%20%28by%20ref%29))
  (bind _self self)
  (bind _returnvalue (Transformation|GetActorLocation _self))
  (bind _asbp_ninja (Utilities|Casting|CastToBP_Ninja OtherActor))
  (if (Variables|Default|GetActive?)
    (Widget|SetVisibility (Variables|/Game/Widgets/HUD.HUD_C|GetIcon_Key (Variables|/Game/Characters/Ninja/BPs/Character/BP_Ninja.BP_Ninja_C|GetHUD _asbp_ninja)) "Collapsed")
    (Audio|PlaySoundatLocation "/Game/Sounds/Stone_Door_Cue.Stone_Door_Cue" _returnvalue "0, 0, 0" 1.0 1.0 0.0 0 0 0 0)
    (bind _movimiento_puertas (Timeline|Timeline Play)
      (:Update
        (Transformation|SetRelativeLocation (Variables|Default|GetStaticMesh) (Math|Vector|MakeVector (* _movimiento_puertas -1.0) 0.0 0.0) false false)
        (Transformation|SetRelativeLocation (Variables|Default|GetHoja_Dcha) (Math|Vector|MakeVector _movimiento_puertas 0.0 0.0) false false)))
    (else
      (Audio|PlaySoundatLocation "/Game/Sounds/CUE_Interact_Sound.CUE_Interact_Sound" _returnvalue "0, 0, 0" 1.0 1.0 0.0 0 0 0 0)
      (Development|SetHiddeninGame (Variables|Default|GetTextRender) false false))))

(event OnComponentEndOverlap(Box)
  (params (OverlappedComponent :type Primitive%20Component%20Object%20Reference) (OtherActor :type Actor%20Object%20Reference) (OtherComp :type Primitive%20Component%20Object%20Reference) (OtherBodyIndex :type Integer))
  (Utilities|Casting|CastToBP_Ninja OtherActor)
  (if (Variables|Default|GetActive?)
    (Audio|PlaySoundatLocation "/Game/Sounds/Stone_Door_Cue.Stone_Door_Cue" (Transformation|GetActorLocation self) "0, 0, 0" 1.0 1.0 0.0 0 0 0 0)
    (bind _movimiento_puertas (Timeline|Timeline Reverse)
      (:Update
        (Transformation|SetRelativeLocation (Variables|Default|GetStaticMesh) (Math|Vector|MakeVector (* _movimiento_puertas -1.0) 0.0 0.0) false false)
        (Transformation|SetRelativeLocation (Variables|Default|GetHoja_Dcha) (Math|Vector|MakeVector _movimiento_puertas 0.0 0.0) false false)))
    (else
      (Development|SetHiddeninGame (Variables|Default|GetTextRender) true false))))

(event EventInteraction
  (Variables|Default|SetActive? true))

(fn ConstructionScript
  (|CallParentFunction))