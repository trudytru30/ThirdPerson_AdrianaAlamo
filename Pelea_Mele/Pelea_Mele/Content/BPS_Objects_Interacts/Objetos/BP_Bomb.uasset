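; Bomb pickup that spins in the world and is collected when BP_Ninja overlaps its box.
; Each overlap increments the ninja's BombCount, destroying the pickup if the count is within a small limit.
; Otherwise it plays a sound and shows a widget until overlap ends, though the count has already been incremented.
; A Timeline started from Tick drives mesh roll and yaw, replaying after a brief delay.
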(event OnComponentBeginOverlap(Box)
  (params (OverlappedComponent :type Primitive%20Component%20Object%20Reference) (OtherActor :type Actor%20Object%20Reference) (OtherComp :type Primitive%20Component%20Object%20Reference) (OtherBodyIndex :type Integer) (bFromSweep :type Boolean) (SweepResult :type Hit%20Result%20Structure%20%28by%20ref%29))
  (bind _asbp_ninja (Utilities|Casting|CastToBP_Ninja OtherActor))
  (bind _result (Math|Integer|IncrementInt (Variables|/Game/Characters/Ninja/BPs/Character/BP_Ninja.BP_Ninja_C|GetBombCount _asbp_ninja))
    (:%20%20
      (if (<= _result 3)
        (Actor|DestroyActor)
        (else
          (Audio|PlaySoundatLocation "/Game/Sounds/Floating_UI_Close-002.Floating_UI_Close-002" (Transformation|GetActorLocation) "0, 0, 0" 1.0 1.0 0.0 0 0 0 0)
          (Rendering|SetVisibility (Variables|Default|GetWidget) true false))))))

(event OnComponentEndOverlap(Box)
  (params (OverlappedComponent :type Primitive%20Component%20Object%20Reference) (OtherActor :type Actor%20Object%20Reference) (OtherComp :type Primitive%20Component%20Object%20Reference) (OtherBodyIndex :type Integer))
  (Rendering|SetVisibility (Variables|Default|GetWidget) false false))

(event Collision|EventActorBeginOverlap
  (params (OtherActor :type Actor%20Object%20Reference)))

(event EventTick
  (params (DeltaSeconds :type Float%20%28single-precision%29))
  (bind _newtrack_0 (Timeline|Timeline Play)
    (:Update
      (Transformation|SetRelativeRotation (Variables|Default|GetStaticMesh) (Math|Rotator|MakeRotator _newtrack_0 0.0 _newtrack_0) false false))
    (:Finished
      (Utilities|FlowControl|Delay 0.1)
      (Timeline|Timeline PlayFromStart))))

(fn ConstructionScript)