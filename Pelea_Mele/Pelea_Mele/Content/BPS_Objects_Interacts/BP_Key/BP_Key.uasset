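; BP_Key is a key pickup that the ninja player collects by touching it.
; On overlap with BP_Ninja, it calls InteractionMessage on the BP_Door returned by GetActorOfClass, so it targets a single door found by class.
; It then reveals the key icon on the ninja's HUD, plays a UI sound at its location and destroys itself.
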(event EventBeginPlay
  (|CallParentFunction) ; This node is disabled and will not be called.\nDrag off pins to build functionality.
)

(event EventTick
  (params (DeltaSeconds :type Float%20%28single-precision%29))
  (|CallParentFunction DeltaSeconds) ; This node is disabled and will not be called.\nDrag off pins to build functionality.
)

(event Collision|EventActorBeginOverlap
  (params (OtherActor :type Actor%20Object%20Reference))
  ;[1 1 1] Comment
  (bind _asbp_ninja (Utilities|Casting|CastToBP_Ninja OtherActor))
  (bind _returnvalue (Actor|GetActorOfClass "/Game/BPS_Objects_Interacts/BP_Door/BP_Door.BP_Door_C"))
  (Class|BPIInteract|Interaction(Message) _returnvalue)
  (Widget|SetVisibility (Variables|/Game/Widgets/HUD.HUD_C|GetIcon_Key (Variables|/Game/Characters/Ninja/BPs/Character/BP_Ninja.BP_Ninja_C|GetHUD _asbp_ninja)) "HitTestInvisible")
  (Audio|PlaySoundatLocation "/Game/Sounds/Floating_UI_Close-002.Floating_UI_Close-002" (Transformation|GetActorLocation) "0, 0, 0" 1.0 1.0 0.0 0 0 0 0)
  (Actor|DestroyActor))

(fn ConstructionScript
  (|CallParentFunction))