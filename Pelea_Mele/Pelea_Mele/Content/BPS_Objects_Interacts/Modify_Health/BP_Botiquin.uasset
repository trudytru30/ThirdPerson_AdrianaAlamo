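; BP_Botiquin is a health pickup (first-aid kit) that offers healing to any actor overlapping it.
; It sends AddHealth through the AddHealthMessage call and branches on the returned CanTake.
; Accepted pickups play a sound and destroy themselves after a short delay.
; Refusals show the returned PrintText on a TextRender, call RotateText and play an interact sound, and ending overlap hides the text.
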(event EventBeginPlay
  (|CallParentFunction) ; This node is disabled and will not be called.\nDrag off pins to build functionality.
)

(event EventTick
  (params (DeltaSeconds :type Float%20%28single-precision%29))
  (|CallParentFunction DeltaSeconds) ; This node is disabled and will not be called.\nDrag off pins to build functionality.
)

(event Collision|EventActorEndOverlap
  (params (OtherActor :type Actor%20Object%20Reference))
  (Development|SetHiddeninGame (Variables|Default|GetTextRender) true false))

(event Collision|EventActorBeginOverlap
  (params (OtherActor :type Actor%20Object%20Reference))
  (bind _textrender (Variables|Default|GetTextRender))
  (bind (_cantake_ _printtext) (Class|BPIInteract|AddHealth(Message) OtherActor (Variables|Default|GetAdd%20Health)))
  (if _cantake_
    (Audio|PlaySoundatLocation "/Game/Sounds/Potion-pickup.Potion-pickup" (Transformation|GetActorLocation self) "0, 0, 0" 1.0 1.0 0.0 0 0 0 0)
    (Utilities|FlowControl|Delay 0.3)
    (Actor|DestroyActor)
    (else
      (Rendering|Components|TextRender|SetText (Variables|Default|GetTextRender) _printtext)
      (Development|SetHiddeninGame _textrender false false)
      (CallFunction|RotateText _textrender)
      (Audio|PlaySoundatLocation "/Game/Sounds/CUE_Interact_Sound.CUE_Interact_Sound" (Transformation|GetWorldLocation _textrender) "0, 0, 0" 1.0 1.0 0.0 0 0 0 0))))

(fn ConstructionScript
  (|CallParentFunction))