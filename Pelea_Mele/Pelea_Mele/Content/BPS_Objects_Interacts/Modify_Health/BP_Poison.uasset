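; BP_Poison is a poison pickup that damages whatever overlaps it.
; On overlap it sends the LossHealth amount to the other actor through the LossHealthMessage interface call.
; It then plays the potion pickup sound at its location and destroys itself after a short delay.
; The overlapping actor is not filtered, and BeginPlay and Tick are unused.
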(event EventBeginPlay
  (|CallParentFunction) ; This node is disabled and will not be called.\nDrag off pins to build functionality.
)

(event EventTick
  (params (DeltaSeconds :type Float%20%28single-precision%29))
  (|CallParentFunction DeltaSeconds) ; This node is disabled and will not be called.\nDrag off pins to build functionality.
)

(event Collision|EventActorBeginOverlap
  (params (OtherActor :type Actor%20Object%20Reference))
  (Class|BPIInteract|LossHealth(Message) OtherActor (Variables|Default|GetLoss%20Health))
  (Audio|PlaySoundatLocation "/Game/Sounds/Potion-pickup.Potion-pickup" (Transformation|GetActorLocation self) "0, 0, 0" 1.0 1.0 0.0 0 0 0 0)
  (Utilities|FlowControl|Delay 0.3)
  (Actor|DestroyActor))

(fn ConstructionScript
  (|CallParentFunction))