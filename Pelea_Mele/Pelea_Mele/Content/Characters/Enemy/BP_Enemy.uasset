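; BP_Enemy is an AI enemy character that the ninja player can stealth-attack and that fights back with melee.
; VictimBox overlap toggles the player's sneak-attack state and the blackboard's under-attack flag.
; Tick maps doubt, alert and detected flags to widget icons, updates the health bar, and calls RunBehaviorTree at zero health.
; Montage notify functions toggle DamageArea collision, with a DoOnce limiting player damage to one hit per swing.
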(event OnComponentBeginOverlap(VictimBox)
  (params (OverlappedComponent :type Primitive%20Component%20Object%20Reference) (OtherActor :type Actor%20Object%20Reference) (OtherComp :type Primitive%20Component%20Object%20Reference) (OtherBodyIndex :type Integer) (bFromSweep :type Boolean) (SweepResult :type Hit%20Result%20Structure%20%28by%20ref%29))
  ;[1 1 1] Activa el modo sneaking del player al entrar en el rango que puede ejecutarlo y seteamos el valor UnderAttack
  (if (not (Variables|Default|GetDead))
    ;;[1 1 1] Seteamos las variables necesarias en el player
    (bind _asbp_ninja (Utilities|Casting|CastToBP_Ninja OtherActor))
    (Variables|/Game/Characters/Ninja/BPs/Character/BP_Ninja.BP_Ninja_C|SetVictim _asbp_ninja self)
    (Variables|/Game/Characters/Ninja/BPs/Character/BP_Ninja.BP_Ninja_C|Setsneaking? _asbp_ninja true)
    (Variables|/Game/Characters/Ninja/BPs/Character/BP_Ninja.BP_Ninja_C|SetbCanAttack _asbp_ninja true)
    (Variables|Default|SetbUnderAttack true)
    (AI|Components|Blackboard|SetValueasBool (AI|GetBlackboard 0) (Utilities|Name|MakeLiteralName "bUnderAttack") true)))

(event OnComponentEndOverlap(VictimBox)
  (params (OverlappedComponent :type Primitive%20Component%20Object%20Reference) (OtherActor :type Actor%20Object%20Reference) (OtherComp :type Primitive%20Component%20Object%20Reference) (OtherBodyIndex :type Integer))
  ;[1 1 1] Activa el modo sneaking del player al entrar en el rango que puede ejecutarlo y seteamos el valor UnderAttack
  (if (not (Variables|Default|GetDead))
    ;;[1 1 1] Seteamos las variables necesarias en el player
    (bind _asbp_ninja (Utilities|Casting|CastToBP_Ninja OtherActor))
    (Variables|/Game/Characters/Ninja/BPs/Character/BP_Ninja.BP_Ninja_C|SetVictim _asbp_ninja 0)
    (Variables|/Game/Characters/Ninja/BPs/Character/BP_Ninja.BP_Ninja_C|Setsneaking? _asbp_ninja false)
    (Variables|/Game/Characters/Ninja/BPs/Character/BP_Ninja.BP_Ninja_C|SetbCanAttack _asbp_ninja false)
    (Variables|Default|SetbUnderAttack false)
    (AI|Components|Blackboard|SetValueasBool (AI|GetBlackboard 0) (Utilities|Name|MakeLiteralName "bUnderAttack") false)))

(event OnComponentBeginOverlap(DamageArea)
  (params (OverlappedComponent :type Primitive%20Component%20Object%20Reference) (OtherActor :type Actor%20Object%20Reference) (OtherComp :type Primitive%20Component%20Object%20Reference) (OtherBodyIndex :type Integer) (bFromSweep :type Boolean) (SweepResult :type Hit%20Result%20Structure%20%28by%20ref%29))
  ;[1 1 1] Enemy Attack
  ;;[1 1 1] Si collisiona con el player hace daño
  (bind _asbp_ninja (Utilities|Casting|CastToBP_Ninja OtherActor))
  (Utilities|FlowControl|DoOnce false
    (:Completed
      (Animation|PlayAnimMontage _asbp_ninja "/Game/Characters/Ninja/Animations/AM_HitReact.AM_HitReact" 1.0 "None")
      (bind _asbp_ninja_2 (Utilities|Casting|CastToBP_Ninja (Game|Player|GetPlayerPawn 0)))
      (Default|LossHealth _asbp_ninja_2 10))))

(event Custom|Attack
  ;[1 1 1] Enemy Attack
  (Utilities|FlowControl|DoOnce false :!label _label
    (:Completed
      (Animation|PlayAnimMontage "/Game/Characters/Enemy/Animations/Anim/AM_EnemyAttack.AM_EnemyAttack" 1.0 "None")
      (Utilities|FlowControl|Delay 0.5)
      (goto _label Reset))))

(event EventBeginPlay
  ;[1 1 1] Sistema de visualizacion de iconos en función de la accioón que este realizando
  (bind _aswbp_enemy_icon (Utilities|Casting|CastToWBP_EnemyIcon (UserInterface|GetUserWidgetObject (Variables|Default|GetWidgetIcons))))
  (Variables|Default|SetEnemy%20Icon _aswbp_enemy_icon)
  (Variables|Default|SetHealth (Variables|Default|GetMax_Health))
  (bind _aswbp_enemy_health_bar (Utilities|Casting|CastToWBP_EnemyHealthBar (UserInterface|GetUserWidgetObject (Variables|Default|GetHealthBar))))
  (Variables|Default|SetHealthBarWidget _aswbp_enemy_health_bar))

(event EventTick
  (params (DeltaSeconds :type Float%20%28single-precision%29))
  (bind _enemy_icon (Variables|Default|GetEnemy%20Icon))
  (bind _enemy_icon_2 (Variables|Default|GetEnemy%20Icon))
  (bind _enemy_icon_3 (Variables|Default|GetEnemy%20Icon))
  (bind _enemy_icon_4 (Variables|Default|GetEnemy%20Icon))
  (Utilities|FlowControl|Sequence
    (:then_0
      ;[1 1 1] Sistema de visualizacion de iconos en función de la accioón que este realizando
      (if (not (Variables|Default|GetDead))
        (if (Variables|Default|GetbDuda)
          (Variables|/Script/UMG.Widget|SetVisibility (Variables|/Game/Widgets/WBP_EnemyIcon.WBP_EnemyIcon_C|GetAlert _enemy_icon_2) "Collapsed")
          (Variables|/Script/UMG.Widget|SetVisibility (Variables|/Game/Widgets/WBP_EnemyIcon.WBP_EnemyIcon_C|GetDetected _enemy_icon_2) "Collapsed")
          (Variables|/Script/UMG.Widget|SetVisibility (Variables|/Game/Widgets/WBP_EnemyIcon.WBP_EnemyIcon_C|GetDuda _enemy_icon_2) "HitTestInvisible")
          (elif (Variables|Default|GetbAlert)
            (Variables|/Script/UMG.Widget|SetVisibility (Variables|/Game/Widgets/WBP_EnemyIcon.WBP_EnemyIcon_C|GetAlert _enemy_icon_3) "HitTestInvisible")
            (Variables|/Script/UMG.Widget|SetVisibility (Variables|/Game/Widgets/WBP_EnemyIcon.WBP_EnemyIcon_C|GetDetected _enemy_icon_3) "Collapsed")
            (Variables|/Script/UMG.Widget|SetVisibility (Variables|/Game/Widgets/WBP_EnemyIcon.WBP_EnemyIcon_C|GetDuda _enemy_icon_3) "Collapsed")
            (elif (Variables|Default|GetbDetected)
              (Variables|/Script/UMG.Widget|SetVisibility (Variables|/Game/Widgets/WBP_EnemyIcon.WBP_EnemyIcon_C|GetAlert _enemy_icon_4) "Collapsed")
              (Variables|/Script/UMG.Widget|SetVisibility (Variables|/Game/Widgets/WBP_EnemyIcon.WBP_EnemyIcon_C|GetDetected _enemy_icon_4) "HitTestInvisible")
              (Variables|/Script/UMG.Widget|SetVisibility (Variables|/Game/Widgets/WBP_EnemyIcon.WBP_EnemyIcon_C|GetDuda _enemy_icon_4) "Collapsed")
              (else
                (Variables|/Script/UMG.Widget|SetVisibility (Variables|/Game/Widgets/WBP_EnemyIcon.WBP_EnemyIcon_C|GetAlert _enemy_icon) "Collapsed")
                (Variables|/Script/UMG.Widget|SetVisibility (Variables|/Game/Widgets/WBP_EnemyIcon.WBP_EnemyIcon_C|GetDetected _enemy_icon) "Collapsed")
                (Variables|/Script/UMG.Widget|SetVisibility (Variables|/Game/Widgets/WBP_EnemyIcon.WBP_EnemyIcon_C|GetDuda _enemy_icon) "Collapsed")))))))
    (:then_1
      (if (< (Variables|Default|GetHealth) (Variables|Default|GetMax_Health))
        (Rendering|SetVisibility (Variables|Default|GetHealthBar) true false)
        (Progress|SetPercent (Variables|/Game/Widgets/WBP_EnemyHealthBar.WBP_EnemyHealthBar_C|GetHealthBar (Variables|Default|GetHealthBarWidget)) (/ (Variables|Default|GetHealth) (Variables|Default|GetMax_Health)))
        (if (<= (Variables|Default|GetHealth) 0.0)
          (bind _asai_controller_enemy (Utilities|Casting|CastToAI_ControllerEnemy (AI|GetAIController 0)))
          (AI|RunBehaviorTree _asai_controller_enemy))))))

(event EventAttackStartFunction
  ;[1 1 1] Enemy Attack
  ;;[1 1 1] Funcion lanzada desde el notify del montage de ataque, seteamos las colisiones para que pueda golpear al player
  (Collision|SetCollisionProfileName (Variables|Default|GetDamageArea) "OverlapAll" true :!class /Script/Engine.PrimitiveComponent))

(event EventAttackEndFunction
  ;[1 1 1] Enemy Attack
  ;;[1 1 1] Funcion lanzada desde el notify del montage de ataque, seteamos las colisiones a noCollision
  (Collision|SetCollisionProfileName (Variables|Default|GetDamageArea) "NoCollision" true :!class /Script/Engine.PrimitiveComponent)
  ;;[1 1 1] Si collisiona con el player hace daño
  (Utilities|FlowControl|DoOnce false) ; enters at Reset
)

(fn ConstructionScript)