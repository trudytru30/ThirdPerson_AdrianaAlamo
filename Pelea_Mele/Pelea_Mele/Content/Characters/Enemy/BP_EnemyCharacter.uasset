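; Enemy character Blueprint that shows the enemy's awareness state and health through widget components.
; On BeginPlay it caches both widgets and max health, hides all icons and binds to the EnemyAIController's awareness-change event.
; That event shows only the icon matching Doubt, Alert or Detected.
; Tick polls HealthComp, revealing and updating the health bar while health is below maximum.
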(event Custom|Show%20Widget
  (params (NewState :type EAwarenessState%20Enum :default "Doubt"))
  (bind _enemy_icon (Variables|Default|GetEnemy%20Icon))
  (bind _enemy_icon_2 (Variables|Default|GetEnemy%20Icon))
  (bind _enemy_icon_3 (Variables|Default|GetEnemy%20Icon))
  (switch Utilities|FlowControl|Switch|SwitchonEAwarenessState NewState
    (:Doubt
      (Variables|/Script/UMG.Widget|SetVisibility (Variables|/Game/Widgets/WBP_EnemyIcon.WBP_EnemyIcon_C|GetAlert _enemy_icon) "Collapsed")
      (Variables|/Script/UMG.Widget|SetVisibility (Variables|/Game/Widgets/WBP_EnemyIcon.WBP_EnemyIcon_C|GetDetected _enemy_icon) "Collapsed")
      (Variables|/Script/UMG.Widget|SetVisibility (Variables|/Game/Widgets/WBP_EnemyIcon.WBP_EnemyIcon_C|GetDuda _enemy_icon) "HitTestInvisible"))
    (:Alert
      (Variables|/Script/UMG.Widget|SetVisibility (Variables|/Game/Widgets/WBP_EnemyIcon.WBP_EnemyIcon_C|GetAlert _enemy_icon_2) "HitTestInvisible")
      (Variables|/Script/UMG.Widget|SetVisibility (Variables|/Game/Widgets/WBP_EnemyIcon.WBP_EnemyIcon_C|GetDetected _enemy_icon_2) "Collapsed")
      (Variables|/Script/UMG.Widget|SetVisibility (Variables|/Game/Widgets/WBP_EnemyIcon.WBP_EnemyIcon_C|GetDuda _enemy_icon_2) "Collapsed"))
    (:Detected
      (Variables|/Script/UMG.Widget|SetVisibility (Variables|/Game/Widgets/WBP_EnemyIcon.WBP_EnemyIcon_C|GetAlert _enemy_icon_3) "Collapsed")
      (Variables|/Script/UMG.Widget|SetVisibility (Variables|/Game/Widgets/WBP_EnemyIcon.WBP_EnemyIcon_C|GetDetected _enemy_icon_3) "HitTestInvisible")
      (Variables|/Script/UMG.Widget|SetVisibility (Variables|/Game/Widgets/WBP_EnemyIcon.WBP_EnemyIcon_C|GetDuda _enemy_icon_3) "Collapsed"))))

(event EventBeginPlay
  (bind _aswbp_enemy_icon (Utilities|Casting|CastToWBP_EnemyIcon (UserInterface|GetUserWidgetObject (Variables|Default|GetWidgetIcons))))
  (Variables|Default|SetEnemy%20Icon _aswbp_enemy_icon)
  (bind _returnvalue (Class|HealthComponent|GetMaxHealt (Variables|Default|GetHealthComp)))
  (Variables|Default|SetMaxHealth _returnvalue)
  (bind _aswbp_enemy_health_bar (Utilities|Casting|CastToWBP_EnemyHealthBar (UserInterface|GetUserWidgetObject (Variables|Default|GetHealthBar))))
  (Variables|Default|SetHealth%20Bar _aswbp_enemy_health_bar)
  (bind _asenemy_aicontroller (Utilities|Casting|CastToEnemyAIController (Pawn|GetController (Class|PawnMovementComponent|GetPawnOwner (Variables|Character|GetCharacterMovement)))))
  (EventDispatchers|BindEventtoOnAwarenessStateChanged _asenemy_aicontroller (delegate Custom|Show%20Widget))
  (Variables|/Script/UMG.Widget|SetVisibility (Variables|/Game/Widgets/WBP_EnemyIcon.WBP_EnemyIcon_C|GetAlert (Variables|Default|GetEnemy%20Icon)) "Collapsed")
  (Variables|/Script/UMG.Widget|SetVisibility (Variables|/Game/Widgets/WBP_EnemyIcon.WBP_EnemyIcon_C|GetDetected (Variables|Default|GetEnemy%20Icon)) "Collapsed")
  (Variables|/Script/UMG.Widget|SetVisibility (Variables|/Game/Widgets/WBP_EnemyIcon.WBP_EnemyIcon_C|GetDuda (Variables|Default|GetEnemy%20Icon)) "Collapsed"))

(event EventTick
  (params (DeltaSeconds :type Float%20%28single-precision%29))
  (bind _returnvalue (Class|HealthComponent|GetCurrentHealt (Variables|Default|GetHealthComp)))
  (bind _output_get (Variables|Default|SetCurrentHealth _returnvalue))
  (if (< _output_get (Variables|Default|GetMaxHealth))
    (Rendering|SetVisibility (Variables|Default|GetHealthBar) true false)
    (Progress|SetPercent (Variables|/Game/Widgets/WBP_EnemyHealthBar.WBP_EnemyHealthBar_C|GetHealthBar (Variables|Default|GetHealth%20Bar)) (/ (Variables|Default|GetCurrentHealth) (Variables|Default|GetMaxHealth)))))

(fn ConstructionScript)