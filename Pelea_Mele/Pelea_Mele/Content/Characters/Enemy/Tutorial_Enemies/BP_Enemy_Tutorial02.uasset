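; BP_Enemy_Tutorial02 is a tutorial enemy character variant built on a parent enemy Blueprint.
; On BeginPlay it runs the parent setup, then hides its health bar.
; It then casts its controller to EnemyAIController and disables the sight sense on the perception component, so it cannot detect targets by vision.
; Tick and construction only defer to the parent.
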(event EventBeginPlay
  (|CallParentFunction)
  (Rendering|SetVisibility (Variables|Default|GetHealthBar) false false)
  (bind _asenemy_aicontroller (Utilities|Casting|CastToEnemyAIController (AI|GetAIController 0)))
  (Class|AIPerceptionComponent|SetSenseEnabled (Variables|/Script/PeleaMelee.EnemyAIController|GetPerceptionComp _asenemy_aicontroller) "/Script/AIModule.AISense_Sight" false))

(event Collision|EventActorBeginOverlap
  (params (OtherActor :type Actor%20Object%20Reference)))

(event EventTick
  (params (DeltaSeconds :type Float%20%28single-precision%29))
  (|CallParentFunction DeltaSeconds))

(fn ConstructionScript
  (|CallParentFunction))